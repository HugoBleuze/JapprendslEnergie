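; BP_Trash is a trash prop that picks a random look and destroys itself when overlapped.
; On BeginPlay it applies a random material from ListofPoubelle to its Cube mesh.
; An overlap on Box1 destroys the actor, prints a debug "Hello" and spawns a scaled-up steam emitter at its location.
; The overlap has no filter on the other actor, and its sound spawn call has no sound assigned.
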(event OnComponentBeginOverlap(Box1)
  (params (OverlappedComponent :type Primitive%20Component%20Object%20Reference) (OtherActor :type Actor%20Object%20Reference) (OtherComp :type Primitive%20Component%20Object%20Reference) (OtherBodyIndex :type Integer) (bFromSweep :type Boolean) (SweepResult :type Hit%20Result%20Structure%20%28by%20ref%29))
  (bind _returnvalue (Transformation|GetActorLocation))
  (Actor|DestroyActor)
  (Development|PrintString "Hello")
  (Effects|SpawnEmitteratLocation "/Game/StarterContent/Particles/P_Steam_Lit.P_Steam_Lit" _returnvalue "0, 0, 0" "5.000000,5.000000,5.000000")
  (Audio|SpawnSoundatLocation 0 _returnvalue "0, 0, 0" 1.0 1.0 0.0 0 0))

(event EventBeginPlay
  (bind _listofpoubelle (Variables|Default|GetListofPoubelle))
  (Rendering|Material|SetMaterial (Variables|Default|Getcube) 0 (Utilities|Array|Get(acopy) _listofpoubelle (Math|Random|RandomIntegerinRange 0 (- (Utilities|Array|Length _listofpoubelle) 1)))))

(fn ConstructionScript)